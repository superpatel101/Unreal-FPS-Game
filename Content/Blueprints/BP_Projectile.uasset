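; BP_Projectile is a timed explosive actor that detonates one second after BeginPlay, with no impact trigger in its graph.
; Explode spawns the explosion particle, applies full radial damage within DamageRadius credited to the instigator's controller, then destroys the actor.
; A debug sphere is drawn after the destroy call, using a hardcoded radius independent of DamageRadius.
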(event Custom|Explode
  (bind _returnvalue (Transformation|GetActorLocation))
  (Effects|SpawnEmitteratLocation "/Game/WeaponEffects/Explosion/P_Explosion.P_Explosion" _returnvalue)
  (Game|Damage|ApplyRadialDamage 1e+02 _returnvalue (Variables|Default|GetDamage%20Radius) 0 0 self (Game|GetInstigatorController) true "ECC_Visibility")
  (Actor|DestroyActor)
  (Rendering|Debug|DrawDebugSphere _returnvalue 4e+02 12 "(R=1.000000,G=0.664457,B=0.000000,A=1.000000)" 2.0 2.0))

(event EventBeginPlay
  (Utilities|FlowControl|Delay 1.0)
  (CallFunction|Explode))

(event Collision|EventActorBeginOverlap
  (params (OtherActor :type Actor%20Object%20Reference)))

(event EventTick
  (params (DeltaSeconds :type Float%20%28single-precision%29)))

(fn ConstructionScript)